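; AI controller for the house owner enemy, driving it through the HouseOwner_BT behavior tree.
; On BeginPlay it runs the tree and copies the locations of the pawn's four patrol point actors into blackboard vectors.
; Perception updates toggle PlayerActorKey for each updated actor, clearing it if already set and otherwise storing that actor, without checking actor type or sensing state.
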(event OnPerceptionUpdated(AIPerception)
  (params (UpdatedActors :type Array%20of%20Actor%20Object%20References))
  (for _array_element UpdatedActors
    (CallFunction|CheckPlayerActor _array_element)))

(event EventBeginPlay
  (AI|RunBehaviorTree "/Game/Enemy/HouseOwner_BT.HouseOwner_BT")
  (CallFunction|InitPatrolPoint))

(event EventTick
  (params (DeltaSeconds :type Float%20%28single-precision%29)))

(fn ConstructionScript)

(fn CheckPlayerActor
  (params (SensedActor :type Actor%20Object%20Reference))
  (Utilities|IsValid (AI|Components|Blackboard|GetValueasObject (AI|GetBlackboard 0) (Utilities|Name|MakeLiteralName "PlayerActorKey"))
    (:Is%20Valid
      (Development|PrintText "나감")
      (AI|Components|Blackboard|SetValueasObject (AI|GetBlackboard 0) (Utilities|Name|MakeLiteralName "PlayerActorKey") 0))
    (:Is%20Not%20Valid
      (Development|PrintText "들어옴")
      (AI|Components|Blackboard|SetValueasObject (AI|GetBlackboard 0) (Utilities|Name|MakeLiteralName "PlayerActorKey") SensedActor))))

(fn InitPatrolPoint
  (bind _ashouse_owner_bp (Utilities|Casting|CastToHouseOwner_BP (Pawn|GetControlledPawn)))
  (AI|Components|Blackboard|SetValueasVector (AI|GetBlackboard 0) (Utilities|Name|MakeLiteralName "PatrolPoint1") (Transformation|GetActorLocation (Variables|/Game/Enemy/HouseOwner_BP.HouseOwner_BP_C|GetPatrolPoint1 _ashouse_owner_bp)))
  (AI|Components|Blackboard|SetValueasVector (AI|GetBlackboard 0) (Utilities|Name|MakeLiteralName "PatrolPoint2") (Transformation|GetActorLocation (Variables|/Game/Enemy/HouseOwner_BP.HouseOwner_BP_C|GetPatrolPoint2 _ashouse_owner_bp)))
  (AI|Components|Blackboard|SetValueasVector (AI|GetBlackboard 0) (Utilities|Name|MakeLiteralName "PatrolPoint3") (Transformation|GetActorLocation (Variables|/Game/Enemy/HouseOwner_BP.HouseOwner_BP_C|GetPatrolPoint3 _ashouse_owner_bp)))
  (AI|Components|Blackboard|SetValueasVector (AI|GetBlackboard 0) (Utilities|Name|MakeLiteralName "PatrolPoint4") (Transformation|GetActorLocation (Variables|/Game/Enemy/HouseOwner_BP.HouseOwner_BP_C|GetPatrolPoint4 _ashouse_owner_bp))))